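; FPS weapon Blueprint that plays cosmetic shot effects through FireEffect, skipped on dedicated servers.
; It picks the first- or third-person mesh and muzzle, then plays the fire sound and montage.
; Fire, impact and decal helper actors spawn lazily, attach to the weapon, and receive impact data each shot.
; Silenced sound selection matches "Silenc" or "Suppress" in muzzle and barrel attachment object names.
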(event `self.FireEffect`
  (params (ImpactPoint :type "Vector Structure (by ref)") (ImpactNormal :type "Vector Structure (by ref)") (ImpactSurfaceType :type "EPhysicalSurface Enum" :default "SurfaceType_Default") (bIsFirstPerson :type Boolean))
  (bind _is_first_person (`self.Is First Person`))
  (bind (_outcomponent _outsocketname) (`self.GetMuzzleAttachPoint` _is_first_person))
  (bind _returnvalue (`KismetSystemLibrary.GetObjectName` (`self.GetAttachmentInSlot` self (`BlueprintGameplayTagLibrary.MakeLiteralGameplayTag` (struct :`TagName` "Attachment.Slot.Muzzle")))))
  (bind _returnvalue_2 (`KismetSystemLibrary.GetObjectName` (`self.GetAttachmentInSlot` self (`BlueprintGameplayTagLibrary.MakeLiteralGameplayTag` (struct :`TagName` "Attachment.Slot.Barrel")))))
  ; Cache Initial value
  (set `self.Is First Person` bIsFirstPerson)
  (if (not (`KismetSystemLibrary.IsDedicatedServer`))
    (set `self.Impact Points` (`|MakeArray` ImpactPoint))
    (set `self.Impact Normals` (`|MakeArray` ImpactNormal))
    (set `self.Impact Surface Types` (`|MakeArray` ImpactSurfaceType))
    (`|ExecutionSequence`
      (:`then_0`
        ; Cache Initial Mesh
        (if _is_first_person
          (set `self.Skeletal Mesh` (`self.Mesh1P`))
          (else
            (set `self.Skeletal Mesh` (`self.Mesh3P`)))))
      (:`then_1`
        ; Cache Muzzle Position
        (set `self.Muzzle Position` (`SceneComponent.GetSocketLocation` _outcomponent _outsocketname)))
      (:`then_2`
        (`|ExecutionSequence`
          (:`then_0`
            ; Only Spawm Calling Yet
            (`/Engine/EditorBlueprintResources/StandardMacros.IsValid` (`self.WeaponFire`)
              (:`Is Valid`
                _)
              (:`Is Not Valid`
                (bind _returnvalue_3 (`|SpawnActorFromClass` "/Game/Effects/Blueprints/B_WeaponFire.B_WeaponFire_C" (`KismetMathLibrary.MakeTransform` (0.0 0.0 0.0)) "Undefined" "OverrideRootScale" null (`self.Skeletal Mesh`) true (`self.Shell Eject System`) true (`self.Muzzle Flash System`) true (`self.Tracer System`) (`self.Shell Eject Mesh`) null))
                (bind _output_get (set `self.WeaponFire` _returnvalue_3))
                (`self.K2_AttachToComponent` _output_get _outcomponent _outsocketname "KeepRelative" "KeepRelative" "KeepRelative" true)))
            ; Set Impoertant value before calling fire
            (set `/Game/Effects/Blueprints/B_WeaponFire.ImpactPositions` (`self.Impact Points`) (`self.WeaponFire`))
            (set `/Game/Effects/Blueprints/B_WeaponFire.ImpactNormals` (`self.Impact Normals`) (`self.WeaponFire`))
            (set `/Game/Effects/Blueprints/B_WeaponFire.ImpactSurfaceTypes` (`self.Impact Surface Types`) (`self.WeaponFire`))
            ; Calling Fire
            (`/Game/Effects/Blueprints/B_WeaponFire.Fire` (`self.WeaponFire`) (`self.Is First Person`)))
          (:`then_1`
            (`/Engine/EditorBlueprintResources/StandardMacros.IsValid` (`self.WeaponImpact`)
              (:`Is Valid`
                _)
              (:`Is Not Valid`
                (bind _returnvalue_4 (`|SpawnActorFromClass` "/Game/Effects/Blueprints/B_WeaponImpacts.B_WeaponImpacts_C" (`KismetMathLibrary.MakeTransform` (0.0 0.0 0.0)) "Undefined" "OverrideRootScale" null 500.0 null))
                (bind _output_get_2 (set `self.WeaponImpact` _returnvalue_4))
                (`self.K2_AttachToComponent` _output_get_2 (`self.Skeletal Mesh`) "None" "KeepRelative" "KeepRelative" "KeepRelative" true)))
            ; Set Important Value
            (set `/Game/Effects/Blueprints/B_WeaponImpacts.ImpactPositions` (`self.Impact Points`) (`self.WeaponImpact`))
            (set `/Game/Effects/Blueprints/B_WeaponImpacts.ImpactNormals` (`self.Impact Normals`) (`self.WeaponImpact`))
            (set `/Game/Effects/Blueprints/B_WeaponImpacts.ImpactSurfaceTypes` (`self.Impact Surface Types`) (`self.WeaponImpact`))
            (set `/Game/Effects/Blueprints/B_WeaponImpacts.MuzzlePosition` (`self.Muzzle Position`) (`self.WeaponImpact`))
            ; Fire
            (`/Game/Effects/Blueprints/B_WeaponImpacts.Fire` (`self.WeaponImpact`) (`self.Is First Person`)))
          (:`then_2`
            (`GameplayStatics.PlaySoundAtLocation` (select `bool` (or (or (`KismetStringLibrary.Contains` _returnvalue "Silenc") (`KismetStringLibrary.Contains` _returnvalue "Suppress")) (or (`KismetStringLibrary.Contains` _returnvalue_2 "Silenc") (`KismetStringLibrary.Contains` _returnvalue_2 "Suppress"))) :`false` (`self.WeaponFireSound`) :`true` (`self.WeaponFireSoundSilenced`)) (`self.K2_GetActorLocation`) (struct) 1.0 1.0 0.0 null null null null)
            (`|PlayMontage` (`self.Skeletal Mesh`) (`self.WeaponFireMontage`)))
          (:`then_3`
            ; Spawn Decals
            (`/Engine/EditorBlueprintResources/StandardMacros.IsValid` (`self.WeaponDecals`)
              (:`Is Valid`
                _)
              (:`Is Not Valid`
                (bind _returnvalue_5 (`|SpawnActorFromClass` "/Game/Effects/Blueprints/B_WeaponDecals.B_WeaponDecals_C" (`KismetMathLibrary.MakeTransform` (0.0 0.0 0.0)) "Undefined" "OverrideRootScale" null null))
                (bind _output_get_3 (set `self.WeaponDecals` _returnvalue_5))
                (`self.K2_AttachToComponent` _output_get_3 (`self.Skeletal Mesh`) "None" "KeepRelative" "KeepRelative" "KeepRelative" true)))
            ; Fire Value
            (set `/Game/Effects/Blueprints/B_WeaponDecals.ImpactPositions` (`self.Impact Points`) (`self.WeaponDecals`))
            (set `/Game/Effects/Blueprints/B_WeaponDecals.ImpactNormals` (`self.Impact Normals`) (`self.WeaponDecals`))
            (set `/Game/Effects/Blueprints/B_WeaponDecals.Impact Surface Types` (`self.Impact Surface Types`) (`self.WeaponDecals`))
            (`/Game/Effects/Blueprints/B_WeaponDecals.fire` (`self.WeaponDecals`) (`self.Muzzle Position`))))))))

(fn `IsSilenced`
  (returns (ReturnValue :type Boolean))
  (bind _returnvalue (`KismetSystemLibrary.GetObjectName` (`self.GetAttachmentInSlot` self (`BlueprintGameplayTagLibrary.MakeLiteralGameplayTag` (struct :`TagName` "Attachment.Slot.Muzzle")))))
  (bind _returnvalue_2 (`KismetSystemLibrary.GetObjectName` (`self.GetAttachmentInSlot` self (`BlueprintGameplayTagLibrary.MakeLiteralGameplayTag` (struct :`TagName` "Attachment.Slot.Barrel")))))
  (return (or (or (`KismetStringLibrary.Contains` _returnvalue "Silenc") (`KismetStringLibrary.Contains` _returnvalue "Suppress")) (or (`KismetStringLibrary.Contains` _returnvalue_2 "Silenc") (`KismetStringLibrary.Contains` _returnvalue_2 "Suppress")))))

(fn `UserConstructionScript`)